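; Game mode that keeps the level populated with BP_Target actors placed at TargetPoint locations.
; BeginPlay spawns one target at every TargetPoint, checking the cap of eight only before the loop.
; Tick uses a Delay to refresh the point list about once a second and, while TargetCnt is below the cap, spawns at a random point.
; TargetCnt only increments here, and spawn points are not checked for existing targets.
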(event EventBeginPlay
  ;[1 1 1] 创建UI和生成靶子
  (if (< (Variables|Default|GetTargetCnt) 8)
    (bind _outactors (Actor|GetAllActorsOfClass "/Script/Engine.TargetPoint"))
    (bind _output_get (Variables|Default|SetAllEnemyRefs _outactors))
    (for _array_element _output_get
      (Game|SpawnActorfromClass "/Game/Blueprints/BP_Target.BP_Target_C" (Transformation|GetActorTransform _array_element) "Undefined" 0 0)
      (Math|Integer|IncrementInt (Variables|Default|GetTargetCnt)))))

(event EventTick
  (params (DeltaSeconds :type Float%20%28single-precision%29))
  ;[1 1 1] 更新靶子
  (Utilities|FlowControl|Delay 1.0)
  (bind _outactors (Actor|GetAllActorsOfClass "/Script/Engine.TargetPoint"))
  (bind _output_get (Variables|Default|SetAllEnemyRefs _outactors))
  (if (< (Variables|Default|GetTargetCnt) 8)
    (Utilities|IsValid (Utilities|Array|Get(acopy) _output_get (Math|Random|RandomIntegerinRange 0 (- (Utilities|Array|Length _output_get) 1)))
      (:Is%20Valid
        (Game|SpawnActorfromClass "/Game/Blueprints/BP_Target.BP_Target_C" (Transformation|GetActorTransform (Utilities|Array|Get(acopy) _output_get (Math|Random|RandomIntegerinRange 0 (- (Utilities|Array|Length _output_get) 1)))) "Undefined" 0 0)
        (Math|Integer|IncrementInt (Variables|Default|GetTargetCnt))))))

(fn ConstructionScript)