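; BP_Shell is a physics shell that explodes with an emitter and sound, pushing nearby cubes.
; Its sphere gathers BP_Cube components into HitActor, never removing them.
; Hitting a simulating body, or anything else below a speed threshold, applies impulses to that list and destroys the shell; only the first case recalculates impulse from velocity.
; Each tick, a downward trace scales velocity by the ground BP_phyMart material's AngularDamping, giving per-surface slowdown.
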(event OnComponentBeginOverlap(Sphere)
  (params (OverlappedComponent :type Primitive%20Component%20Object%20Reference) (OtherActor :type Actor%20Object%20Reference) (OtherComp :type Primitive%20Component%20Object%20Reference) (OtherBodyIndex :type Integer) (bFromSweep :type Boolean) (SweepResult :type Hit%20Result%20Structure%20%28by%20ref%29))
  (bind _hitactor (Variables|Default|GetHitActor))
  ;[1 1 1] 检测炮弹范围内的物体
  (if (== (Utilities|GetClass (Components|GetOwner OtherComp)) "/Game/Blueprints/BP_Cube.BP_Cube_C")
    (if (not (Utilities|Array|ContainsItem _hitactor OtherComp))
      (Utilities|Array|Add _hitactor OtherComp))))

(event OnComponentEndOverlap(Sphere)
  (params (OverlappedComponent :type Primitive%20Component%20Object%20Reference) (OtherActor :type Actor%20Object%20Reference) (OtherComp :type Primitive%20Component%20Object%20Reference) (OtherBodyIndex :type Integer))
  ;[1 1 1] 检测炮弹范围内的物体
)

(event EventBeginPlay)

(event Collision|EventActorBeginOverlap
  (params (OtherActor :type Actor%20Object%20Reference)))

(event EventTick
  (params (DeltaSeconds :type Float%20%28single-precision%29))
  (bind _self self)
  (bind _returnvalue (Transformation|GetActorLocation _self))
  ;[1 1 1] 不同材质速度衰减不同
  (bind _outhit (Collision|LineTraceForObjects _returnvalue (- _returnvalue "0, 0,50.000000") (Utilities|Array|MakeArray "ObjectTypeQuery1") false 0 "None"))
  (bind _asbp_phy_mart (Utilities|Casting|CastToBP_phyMart (.physmat _outhit)))
  (Class|PrimitiveComponent|SetAllPhysicsLinearVelocity (Variables|Default|GetStaticMesh) (* (Transformation|GetVelocity) (Variables|/Game/Blueprints/BP_phyMart.BP_phyMart_C|GetAngularDamping _asbp_phy_mart)) false))

(event Collision|EventHit
  (params (MyComp :type Primitive%20Component%20Object%20Reference) (Other :type Actor%20Object%20Reference) (OtherComp :type Primitive%20Component%20Object%20Reference) (bSelfMoved :type Boolean) (HitLocation :type Vector :default "0, 0, 0") (HitNormal :type Vector :default "0, 0, 0") (NormalImpulse :type Vector :default "0, 0, 0") (Hit :type Hit%20Result%20Structure%20%28by%20ref%29))
  (bind _returnvalue (Transformation|GetVelocity))
  (bind _returnvalue_2 (Transformation|GetActorLocation))
  ;[1 1 1] 炮弹爆炸时施加冲量
  (if (Class|SceneComponent|IsAnySimulatingPhysics OtherComp)
    (Variables|Default|SetSpeed (* (Transformation|GetVelocity) 2e+02))
    (for _array_element (Variables|Default|GetHitActor)
      (Physics|AddImpulseatLocation _array_element (Variables|Default|GetSpeed) (Transformation|GetWorldLocation _array_element) "None"))
    (Actor|DestroyActor)
    (Effects|SpawnEmitteratLocation "/Game/Effects/Weapons/Impacts/P_AssaultRifle_IH.P_AssaultRifle_IH" _returnvalue_2 "0, 0, 0" "5.000000,5.000000,5.000000")
    (Audio|SpawnSoundatLocation "/Game/Sound/audio/gunfire.gunfire" _returnvalue_2 "0, 0, 0" 1.0 1.0 0.0 0 0)
    (elif (< (Math|Float|Sqrt (+ (* (.x _returnvalue) (.x _returnvalue)) (* (.y _returnvalue) (.y _returnvalue)) (* (.z _returnvalue) (.z _returnvalue)))) 2e+02)
      (for _array_element_2 (Variables|Default|GetHitActor)
        (Physics|AddImpulseatLocation _array_element_2 (Variables|Default|GetSpeed) (Transformation|GetWorldLocation _array_element_2) "None"))
      (Actor|DestroyActor)
      (Effects|SpawnEmitteratLocation "/Game/Effects/Weapons/Impacts/P_AssaultRifle_IH.P_AssaultRifle_IH" _returnvalue_2 "0, 0, 0" "5.000000,5.000000,5.000000")
      (Audio|SpawnSoundatLocation "/Game/Sound/audio/gunfire.gunfire" _returnvalue_2 "0, 0, 0" 1.0 1.0 0.0 0 0))))

(fn ConstructionScript)